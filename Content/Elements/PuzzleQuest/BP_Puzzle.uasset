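; BP_Puzzle is a rotation-code quest puzzle where interaction turns one of its meshes to match target angles.
; InteractwithPuzzle yaws the given component left or right by RotateValue, then calls CheckCode.
; CheckCode maps three static meshes to indices, comparing relative yaw against the Code array within a small tolerance.
; Results persist in CodeIsGood, and when all entries are true it only prints a quest-passed message.
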(event `/Game/Elements/PuzzleQuest/InteractWithPuzzles.InteractWithPuzzle`
  (params (Component :type "PrimitiveComponent Object Reference") (RotateLeft :type Boolean))
  (`self.Rotate` Component RotateLeft))

(fn `CheckCode`
  (params (Component :type "PrimitiveComponent Object Reference"))
  (locals (SelectedMesh :type Integer) (LocalFailed :type Boolean))
  (bind (_relativerotation_roll _relativerotation_pitch _relativerotation_yaw) (`KismetMathLibrary.BreakRotator` (`SceneComponent.RelativeRotation` Component)))
  (if (== Component (`self.StaticMesh`))
    (set `local.SelectedMesh` 0)
    (`KismetArrayLibrary.Array_Set` (`self.CodeIsGood`) (`local.SelectedMesh`) (`KismetMathLibrary.NearlyEqual_FloatFloat` (`|GetArrayItem` (`self.Code`) (`local.SelectedMesh`)) _relativerotation_yaw 1.0) :!label _label)
    (for _array_element (`self.CodeIsGood`)
      (if (not _array_element)
        (set `local.LocalFailed` true)
        (break)))
    (if (not (`local.LocalFailed`))
      (`KismetSystemLibrary.PrintString` "CODE IS GOOD; QUEST PASSED"))
    (elif (== Component (`self.StaticMesh1`))
      (set `local.SelectedMesh` 1)
      (goto _label)
      (elif (== Component (`self.StaticMesh2`))
        (set `local.SelectedMesh` 2)
        (goto _label)))))

(fn `Rotate`
  (params (Component :type "PrimitiveComponent Object Reference") (RotateLeft :type Boolean))
  (if RotateLeft
    (`SceneComponent.K2_AddRelativeRotation` Component (`KismetMathLibrary.MakeRotator` 0.0 0.0 (* (`self.RotateValue`) -1.0)) false false)
    (else
      (`SceneComponent.K2_AddRelativeRotation` Component (`KismetMathLibrary.MakeRotator` 0.0 0.0 (`self.RotateValue`)) false false)))
  (`self.CheckCode` Component))

(fn `UserConstructionScript`)