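; BP_PuzzleGate is a quest gate that opens once enough items have been collected.
; CollectItem increments the collected count and marks the quest completed when it reaches the maximum.
; OpenDoorCheck compares the count to that maximum and, through a DoOnce, calls OpenDoor.
; OpenDoor plays a timeline that swings the Door component open by interpolating its yaw.
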(event `Open Door`
  (bind (_direction _door_rotation) (`Timeline|Open Door Timeline`)
    (:`Update`
      (`SceneComponent.K2_SetRelativeRotation` (`self.Door`) (`KismetMathLibrary.MakeRotator` 0.0 0.0 (`KismetMathLibrary.Lerp` 0.0 120.0 _door_rotation)) false false))))

(event `Collect Item`
  (`/Engine/EditorBlueprintResources/StandardMacros.IncrementInt` (`self.Current Items Collected`)
    (:`  `
      (if (>= (`self.Current Items Collected`) (`self.Max Item To Collect`))
        (set `self.quest_completed` true)))))

(event `Open Door Check`
  (if (>= (`self.Current Items Collected`) (`self.Max Item To Collect`))
    (`/Engine/EditorBlueprintResources/StandardMacros.DoOnce` false
      (:`Completed`
        (`self.Open Door`)))))

(fn `UserConstructionScript`)